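; BP_SafeZoneVolume is a safe zone volume that makes overlapping actors immune to damage.
; Overlap events clear CanBeDamaged on entry and restore it only once the actor no longer overlaps the volume at all.
; The construction script turns option flags into collision settings: Pawn and Vehicle overlaps for damage protection, WorldStatic object type to disable shooting, and a custom trace channel block for bullets.
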(event OnComponentBeginOverlap(CollisionComponent)
  (params (OverlappedComponent :type Primitive%20Component%20Object%20Reference) (OtherActor :type Actor%20Object%20Reference) (OtherComp :type Primitive%20Component%20Object%20Reference) (OtherBodyIndex :type Integer) (bFromSweep :type Boolean) (SweepResult :type Hit%20Result%20Structure%20%28by%20ref%29))
  (Variables|/Script/Engine.Actor|SetbCanBeDamaged OtherActor false))

(event OnComponentEndOverlap(CollisionComponent)
  (params (OverlappedComponent :type Primitive%20Component%20Object%20Reference) (OtherActor :type Actor%20Object%20Reference) (OtherComp :type Primitive%20Component%20Object%20Reference) (OtherBodyIndex :type Integer))
  (if (not (Collision|IsOverlappingActor self OtherActor :!class /Script/Engine.Actor))
    (Variables|/Script/Engine.Actor|SetbCanBeDamaged OtherActor true)))

(fn ConstructionScript
  (Utilities|FlowControl|Sequence
    (:then_0
      (if (Variables|Default|GetDisableShooting?)
        (Collision|SetCollisionObjectType (Variables|Default|GetCollisionComponent) "ECC_WorldStatic")))
    (:then_1
      (if (Variables|Default|GetDisablePlayerDamage?)
        (Collision|SetCollisionResponsetoChannel (Variables|Default|GetCollisionComponent) "ECC_Pawn" "ECR_Overlap")))
    (:then_2
      (if (Variables|Default|GetDisableVehicleDamage?)
        (Collision|SetCollisionResponsetoChannel (Variables|Default|GetCollisionComponent) "ECC_Vehicle" "ECR_Overlap")))
    (:then_3
      (if (Variables|Default|GetBlockBullets?)
        (Collision|SetCollisionResponsetoChannel (Variables|Default|GetCollisionComponent) "ECC_GameTraceChannel1" "ECR_Block")))))