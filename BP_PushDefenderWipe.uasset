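; Pavlov Push mode helper actor that wipes out the defending team once all of its bomb objectives are destroyed.
; On BeginPlay the server counts the Objectives array and binds to each objective's state-change and team-switch events.
; Each destruction decrements the remaining count, which team switches reset.
; At zero, lethal environmental damage hits every living team 0 pawn in the player array.
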(event Custom|OnSwitchedTeams
  (Variables|Default|SetValidPushBombObjectives (Variables|Default|GetPushBombObjectives)))

(event Custom|OnPushObjectiveStateChanged
  (params (ObjectiveState :type EPushObjectiveState%20Enum :default "Inactive"))
  (switch Utilities|FlowControl|Switch|SwitchonEPushObjectiveState ObjectiveState
    (:Destroyed
      (if (> (Variables|Default|GetValidPushBombObjectives) 0)
        (bind _result (Math|Integer|DecrementInt (Variables|Default|GetValidPushBombObjectives))
          (:%20%20
            (if (<= _result 0)
              (for _array_element (Variables|/Script/Engine.GameStateBase|GetPlayerArray (Game|GetGameState))
                (bind _aspavlov_pawn (Utilities|Casting|CastToPavlovPawn (Variables|/Script/Engine.PlayerState|GetPawnPrivate _array_element)))
                (if (and (== (Variables|/Script/Pavlov.PavlovPawn|GetTeamId _aspavlov_pawn) 0) (not (Class|PavlovPawn|IsDead _aspavlov_pawn)))
                  (Game|Damage|ApplyDamage _aspavlov_pawn 999.0 0 self "/Engine/EngineDamageTypes/DmgTypeBP_Environmental.DmgTypeBP_Environmental_C"))))))))))

(event EventBeginPlay
  (Networking|SwitchHasAuthority
    (:Authority
      (bind _output_get (Variables|Default|SetPushBombObjectives (Utilities|Array|Length (Variables|Default|GetObjectives))))
      (Variables|Default|SetValidPushBombObjectives _output_get)
      (for _array_element (Variables|Default|GetObjectives)
        (EventDispatchers|BindEventtoOnSwitchedTeamsServer _array_element (delegate Custom|OnSwitchedTeams))
        (EventDispatchers|BindEventtoOnPushObjectiveStateChanged _array_element (delegate Custom|OnPushObjectiveStateChanged))))))

(fn ConstructionScript)