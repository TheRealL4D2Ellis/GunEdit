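; Kill volume for Push mode in Pavlov that deals lethal environmental damage to living pawns inside it while its linked bomb objectives remain.
; On the server, it binds to each objective's state and team-switch events.
; The first objective to activate enables collision through a DoOnce and kills pawns already overlapping; later entrants die on overlap.
; Destroying all objectives disables collision, and switching teams resets the count and DoOnce.
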(event OnComponentBeginOverlap(CollisionComponent)
  (params (OverlappedComponent :type Primitive%20Component%20Object%20Reference) (OtherActor :type Actor%20Object%20Reference) (OtherComp :type Primitive%20Component%20Object%20Reference) (OtherBodyIndex :type Integer) (bFromSweep :type Boolean) (SweepResult :type Hit%20Result%20Structure%20%28by%20ref%29))
  (bind _aspavlov_pawn (Utilities|Casting|CastToPavlovPawn OtherActor))
  (if (not (Class|PavlovPawn|IsDead _aspavlov_pawn))
    (Game|Damage|ApplyDamage _aspavlov_pawn 999.0 0 self "/Engine/EngineDamageTypes/DmgTypeBP_Environmental.DmgTypeBP_Environmental_C")))

(event Custom|OnSwitchedTeams
  (Variables|Default|SetValidPushBombObjectives (Variables|Default|GetPushBombObjectives))
  (Utilities|FlowControl|DoOnce false) ; enters at Reset
)

(event Custom|OnPushObjectiveStateChanged
  (params (ObjectiveState :type EPushObjectiveState%20Enum :default "Inactive"))
  (switch Utilities|FlowControl|Switch|SwitchonEPushObjectiveState ObjectiveState
    (:Active
      (Utilities|FlowControl|DoOnce false
        (:Completed
          (Collision|SetCollisionEnabled (Variables|Default|GetCollisionComponent) "QueryOnly")
          (for _array_element (Collision|GetOverlappingActors (Variables|Default|GetCollisionComponent) "/Script/Pavlov.PavlovPawn" :!class /Script/Engine.PrimitiveComponent)
            (bind _aspavlov_pawn (Utilities|Casting|CastToPavlovPawn _array_element))
            (if (not (Class|PavlovPawn|IsDead _aspavlov_pawn))
              (Game|Damage|ApplyDamage _aspavlov_pawn 999.0 0 self "/Engine/EngineDamageTypes/DmgTypeBP_Environmental.DmgTypeBP_Environmental_C"))))))
    (:Destroyed
      (if (> (Variables|Default|GetValidPushBombObjectives) 0)
        (bind _result (Math|Integer|DecrementInt (Variables|Default|GetValidPushBombObjectives))
          (:%20%20
            (if (<= _result 0)
              (Collision|SetCollisionEnabled (Variables|Default|GetCollisionComponent) "NoCollision"))))))))

(event EventBeginPlay
  (Networking|SwitchHasAuthority
    (:Authority
      (bind _output_get (Variables|Default|SetPushBombObjectives (Utilities|Array|Length (Variables|Default|GetObjectives))))
      (Variables|Default|SetValidPushBombObjectives _output_get)
      (for _array_element (Variables|Default|GetObjectives)
        (EventDispatchers|BindEventtoOnSwitchedTeamsServer _array_element (delegate Custom|OnSwitchedTeams))
        (EventDispatchers|BindEventtoOnPushObjectiveStateChanged _array_element (delegate Custom|OnPushObjectiveStateChanged))))))

(fn ConstructionScript)