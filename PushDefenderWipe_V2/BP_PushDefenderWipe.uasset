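; Pavlov Push-mode actor that kills living team 0 players (the defenders) once all its assigned objectives are destroyed.
; On the server it binds to each objective, counts down on Destroyed and resets the count on team switch.
; VolumeRule selects whether lethal environmental damage hits everyone on that team, only those inside, or only those outside tagged volumes.
; Volumes are found at wipe time by a tag built from the first objective's ID.
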(event Custom|OnSwitchedTeams
  (Variables|Default|SetValidPushBombObjectives (Variables|Default|GetPushBombObjectives)))

(event Custom|OnPushObjectiveStateChanged
  (params (ObjectiveState :type EPushObjectiveState%20Enum :default "Inactive"))
  (switch Utilities|FlowControl|Switch|SwitchonEPushObjectiveState ObjectiveState
    (:Destroyed
      (if (> (Variables|Default|GetValidPushBombObjectives) 0)
        (bind _result (Math|Integer|DecrementInt (Variables|Default|GetValidPushBombObjectives))
          (:%20%20
            (if (<= _result 0)
              (switch int (Variables|Default|GetVolumeRule)
                (:0
                  _)
                (:1
                  (bind _outactors (Actor|GetAllActorswithTag (Utilities|String|StringToName (Utilities|String|Append "PushDefenderWipeVolume_Objective" (Utilities|String|ToString(Integer) (Variables|Default|GetObjective%20Id)))) :!label _label))
                  (Variables|Default|Set_Volumes _outactors))
                (:2
                  (goto _label)))
              (for _array_element (Variables|/Script/Engine.GameStateBase|GetPlayerArray (Game|GetGameState))
                (bind _aspavlov_pawn (Utilities|Casting|CastToPavlovPawn (Variables|/Script/Engine.PlayerState|GetPawnPrivate _array_element)))
                (if (and (== (Variables|/Script/Pavlov.PavlovPawn|GetTeamId _aspavlov_pawn) 0) (not (Class|PavlovPawn|IsDead _aspavlov_pawn)))
                  (switch int (Variables|Default|GetVolumeRule)
                    (:0
                      (Game|Damage|ApplyDamage _aspavlov_pawn 999.0 0 self "/Engine/EngineDamageTypes/DmgTypeBP_Environmental.DmgTypeBP_Environmental_C"))
                    (:1
                      (bind _array_element_2 (Utilities|Array|ForEachLoopwithBreak (Variables|Default|Get_Volumes) :!label _label_2)
                        (:LoopBody
                          (if (Collision|IsOverlappingActor _aspavlov_pawn _array_element_2 :!class /Script/Engine.Actor)
                            (Game|Damage|ApplyDamage _aspavlov_pawn 999.0 0 self "/Engine/EngineDamageTypes/DmgTypeBP_Environmental.DmgTypeBP_Environmental_C")
                            (goto _label_2 Break)))))
                    (:2
                      (Variables|Default|SetbVR2Overlap false)
                      (bind _array_element_3 (Utilities|Array|ForEachLoopwithBreak (Variables|Default|Get_Volumes) :!label _label_3)
                        (:LoopBody
                          (if (Collision|IsOverlappingActor _aspavlov_pawn _array_element_3 :!class /Script/Engine.Actor)
                            (Variables|Default|SetbVR2Overlap true)
                            (goto _label_3 Break)))
                        (:Completed
                          (if (not (Variables|Default|GetbVR2Overlap))
                            (Game|Damage|ApplyDamage _aspavlov_pawn 999.0 0 self "/Engine/EngineDamageTypes/DmgTypeBP_Environmental.DmgTypeBP_Environmental_C")))))))))))))))

(event EventBeginPlay
  (Networking|SwitchHasAuthority
    (:Authority
      (bind _output_get (Variables|Default|SetPushBombObjectives (Utilities|Array|Length (Variables|Default|GetObjectives))))
      (Variables|Default|SetValidPushBombObjectives _output_get)
      (for _array_element (Variables|Default|GetObjectives)
        (EventDispatchers|BindEventtoOnSwitchedTeamsServer _array_element (delegate Custom|OnSwitchedTeams))
        (EventDispatchers|BindEventtoOnPushObjectiveStateChanged _array_element (delegate Custom|OnPushObjectiveStateChanged))
        (Utilities|FlowControl|DoOnce false
          (:Completed
            (Variables|Default|SetObjective%20Id (Variables|/Script/PavlovProxy.Pavlov_PushBombObjective|GetObjectiveId _array_element))))))))

(fn ConstructionScript)