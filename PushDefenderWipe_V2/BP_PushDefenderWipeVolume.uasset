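; BP_PushDefenderWipeVolume is a volume actor for a push-mode defender wipe, tagged by the objectives it belongs to.
; Its construction script turns each entry in ObjectiveIds into a unique "PushDefenderWipeVolume_Objective" name tag with the ID appended.
; It then writes that list to the actor's Tags, so each volume is identifiable per objective by tag.
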(fn ConstructionScript
  (if (Utilities|Array|IsNotEmpty (Variables|Default|GetObjectiveIds))
    (for _array_element (Variables|Default|GetObjectiveIds)
      (Utilities|Array|AddUnique (LocalVariables|Get_TagCreation) (Utilities|String|StringToName (Utilities|String|Append "PushDefenderWipeVolume_Objective" (Utilities|String|ToString(Integer) _array_element)))))
    (Variables|Default|SetTags (LocalVariables|Get_TagCreation))))