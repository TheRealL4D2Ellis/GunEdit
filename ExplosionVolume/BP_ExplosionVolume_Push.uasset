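; BP_ExplosionVolume_Push is an explosion volume variant tied to a set of push bomb objectives, with event logic bound on the authority.
; The first objective to become Active starts the parent's explosion timer through a DoOnce, provided undestroyed objectives remain.
; Each Destroyed objective decrements the remaining count, and reaching zero cancels the timer.
; A team switch restores the count and resets the DoOnce.
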(event Custom|OnSwitchedTeams
  (Variables|Default|SetValidPushBombObjectives (Variables|Default|GetPushBombObjectives))
  (Utilities|FlowControl|DoOnce false) ; enters at Reset
)

(event Custom|OnPushObjectiveStateChanged
  (params (ObjectiveState :type EPushObjectiveState%20Enum :default "Inactive"))
  (switch Utilities|FlowControl|Switch|SwitchonEPushObjectiveState ObjectiveState
    (:Active
      (Utilities|FlowControl|DoOnce false
        (:Completed
          (CallFunction|StartExplosionTImer))))
    (:Destroyed
      (if (> (Variables|Default|GetValidPushBombObjectives) 0)
        (bind _result (Math|Integer|DecrementInt (Variables|Default|GetValidPushBombObjectives))
          (:%20%20
            (if (<= _result 0)
              (Utilities|Time|ClearandInvalidateTimerbyHandle (Variables|Default|GetExplosionTimerHandle)))))))))

(event EventBeginPlay
  (Networking|SwitchHasAuthority
    (:Authority
      (bind _output_get (Variables|Default|SetPushBombObjectives (Utilities|Array|Length (Variables|Default|GetObjectives))))
      (Variables|Default|SetValidPushBombObjectives _output_get)
      (for _array_element (Variables|Default|GetObjectives)
        (EventDispatchers|BindEventtoOnSwitchedTeamsServer _array_element (delegate Custom|OnSwitchedTeams))
        (EventDispatchers|BindEventtoOnPushObjectiveStateChanged _array_element (delegate Custom|OnPushObjectiveStateChanged))))))

(fn ConstructionScript
  (|CallParentFunction))

(fn StartExplosionTImer
  (if (> (Variables|Default|GetValidPushBombObjectives) 0)
    (|CallParentFunction)))