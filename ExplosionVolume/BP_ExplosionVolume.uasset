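; Box volume for Pavlov that sets off explosions at random points and random intervals, with optional radial damage.
; An authority-only timer traces down from the volume's top, retrying immediately on a miss or, with AvoidPlayers, when a temporary sphere overlaps a PavlovPawn.
; The Explosion event spawns sound and particles, while damage stays on authority.
; Remote instances show effects only if EnabledLocally and within MaxShowDistance of the VR tracking origin.
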(event Custom|Explosion
  (params (Location :type Vector))
  (Networking|SwitchHasAuthority
    (:Authority
      (CallFunction|SpawnExplosion Location :!label _label))
    (:Remote
      (if (Variables|Default|GetbEnabledLocally)
        (if (not (CallFunction|MaxShowDistanceExceeded))
          (goto _label))))))

(event EventBeginPlay
  (Networking|SwitchHasAuthority
    (:Authority
      (CallFunction|StartExplosionTImer))))

(fn ConstructionScript
  (Variables|Private|SetLocation (Transformation|GetActorLocation))
  (bind _output_get (Variables|Private|SetAreaHalfSize (/ (Variables|Default|GetArea) 2.0)))
  (Components|Box|SetBoxExtent (Variables|Default|GetAreaVolume) _output_get true))

(fn ExplosionTimer
  (bind _location (Variables|Private|GetLocation))
  (bind _areahalfsize (Variables|Private|GetAreaHalfSize))
  (bind _output_get (LocalVariables|SetTraceStart (Math|Random|RandomPointinBoundingBox (Math|Vector|MakeVector (.x _location) (.y _location) (+ (.z _location) (.z _areahalfsize))) (Math|Vector|MakeVector (.x _areahalfsize) (.y _areahalfsize) 1.0)) :!label _label))
  (bind (_outhit _returnvalue) (Collision|LineTraceByChannel _output_get (- _output_get (Math|Vector|MakeVector 0.0 0.0 (.z (Variables|Default|GetArea)))) "TraceTypeQuery1" false 0 "None"))
  (if _returnvalue
    (LocalVariables|SetImpact%20Point (.ImpactPoint (Collision|BreakHitResult _outhit)))
    (if (Variables|Default|GetbAvoidPlayers?)
      (bind _returnvalue_2 (AddComponent|AddSphereComponent false))
      (Components|Sphere|SetSphereRadius _returnvalue_2 (.y (Variables|Damage|GetDamage%20Radius)) true)
      (Transformation|SetWorldLocation _returnvalue_2 (LocalVariables|GetImpact%20Point) false true)
      (if (Utilities|Array|IsEmpty (Collision|GetOverlappingActors _returnvalue_2 "/Script/Pavlov.PavlovPawn" :!class /Script/Engine.PrimitiveComponent))
        (Components|DestroyComponent _returnvalue_2)
        (CallFunction|Explosion (LocalVariables|GetImpact%20Point))
        (CallFunction|StartExplosionTImer)
        (else
          (Components|DestroyComponent _returnvalue_2)
          (goto _label)))
      (else
        (CallFunction|Explosion (LocalVariables|GetImpact%20Point))
        (CallFunction|StartExplosionTImer)))
    (else
      (goto _label))))

(fn MaxShowDistanceExceeded
  (if (!= (Variables|Default|GetMaxShowDistance) 0.0)
    (bind _returnvalue (Class|HeadMountedDisplayFunctionLibrary|GetTrackingtoWorldTransform))
    (return (> (Math|Vector|Distance(Vector) (.location _returnvalue) (Variables|Private|GetLocation)) (Variables|Default|GetMaxShowDistance)))))

(fn SpawnExplosion
  (params (Location :type Vector%20%28by%20ref%29))
  (bind _damage_radius (Variables|Damage|GetDamage%20Radius))
  (bind _base_damage (Variables|Damage|GetBase%20Damage))
  (Audio|PlaySoundatLocation 0 Location "0, 0, 0" 1.0 1.0 0.0 0 0 0 0)
  (Effects|SpawnEmitteratLocation 0 Location)
  (Networking|SwitchHasAuthority
    (:Authority
      (if (Variables|Damage|GetbApplyDamage?)
        (Class|GameplayStatics|ApplyRadialDamagewithFalloff (.x _base_damage) (.y _base_damage) Location (.x _damage_radius) (.y _damage_radius) (Variables|Damage|GetDamage%20Falloff) "/Script/Engine.DamageType" 0 self 0 "ECC_Visibility")))))

(fn StartExplosionTImer
  (bind _frequency__seconds_ (Variables|Default|GetFrequency%20%28Seconds%29))
  (bind _returnvalue (Utilities|Time|SetTimerbyFunctionName 0 "ExplosionTimer" (Math|Random|RandomFloatinRange (.x _frequency__seconds_) (.y _frequency__seconds_))))
  (Variables|Default|SetExplosionTimerHandle _returnvalue))